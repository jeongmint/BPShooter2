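; BP_Enemy2 is an enemy actor that flies in a straight line and destroys itself along with what it hits.
; Tick moves it along its normalized Direction scaled by Speed and delta time, without sweep.
; StaticMesh overlap ignores other BP_Enemy2 actors and destroys both parties otherwise.
; Nothing here sets Direction: FindDirection is empty, and BeginPlay's GetActorOfClass result goes unused.
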(event `self.ReceiveBeginPlay`
  (`GameplayStatics.GetActorOfClass` null))

(event `self.ReceiveTick`
  (params (DeltaSeconds :type "Float (single-precision)"))
  (`self.K2_SetActorLocation` (+ (* (* (`KismetMathLibrary.Normal` (`self.Direction`)) (`self.Speed`)) DeltaSeconds) (`self.K2_GetActorLocation`))))

(event `self.StaticMesh.OnComponentBeginOverlap`
  (params (OverlappedComponent :type "PrimitiveComponent Object Reference") (OtherActor :type "Actor Object Reference") (OtherComp :type "PrimitiveComponent Object Reference") (OtherBodyIndex :type Integer) (bFromSweep :type Boolean) (SweepResult :type "HitResult Structure (by ref)"))
  (cast `/Game/Copy/BP_Enemy2` OtherActor
    (:`CastFailed`
      (`self.K2_DestroyActor` OtherActor)
      (`self.K2_DestroyActor`))))

(fn `FindDirection`)

(fn `UserConstructionScript`)