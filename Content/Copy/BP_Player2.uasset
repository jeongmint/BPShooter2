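; Player-controlled actor that moves in the Y-Z plane and fires bullets, enabling input from player controller 0 at BeginPlay.
; Horizontal and Vertical axis events share one setter that writes the Y and Z components of Direction.
; Tick moves the actor along normalized Direction scaled by Speed and delta time, without sweep.
; Pressing Fire calls CreateBullet, which spawns BP_Bullet2 at the actor's transform, ignoring collisions.
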(event `self.ReceiveBeginPlay`
  (`self.EnableInput` (`GameplayStatics.GetPlayerController` 0)))

(event `InputAction|Fire`
  (params (Key :type "Key Structure"))
  (:`Pressed`
    (`self.CreateBullet`)))

(event `InputAxis|Horizontal`
  (params (AxisValue :type "Float (single-precision)"))
  (set `self.Direction` (`KismetMathLibrary.MakeVector` 0.0 AxisValue (stale `InputAxis|Vertical` AxisValue)) :!label _label))

(event `InputAxis|Vertical`
  (params (AxisValue :type "Float (single-precision)"))
  (goto _label))

(event `self.ReceiveTick`
  (params (DeltaSeconds :type "Float (single-precision)"))
  (`self.K2_SetActorLocation` (+ (* (* (`KismetMathLibrary.Normal` (`self.Direction`)) (`self.Speed`)) DeltaSeconds) (`self.K2_GetActorLocation`))))

(fn `CreateBullet`
  (`|SpawnActorFromClass` "/Game/Copy/BP_Bullet2.BP_Bullet2_C" (`self.GetTransform`) "AlwaysSpawn" "OverrideRootScale" null null))

(fn `UserConstructionScript`)