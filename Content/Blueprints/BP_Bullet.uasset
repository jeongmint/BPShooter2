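; BP_Bullet is a projectile actor that flies straight along world up (+Z) and expires after a short lifespan.
; BeginPlay fixes the Direction vector and sets the lifespan.
; Tick moves the actor by normalized Direction times Speed and delta time, using SetActorLocation without sweep instead of a movement component.
; The overlap event is empty, so the bullet has no hit handling of its own.
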(event `self.ReceiveBeginPlay`
  (set `self. Direction` (`KismetMathLibrary.MakeVector` 0.0 0.0 1.0))
  (`self.SetLifeSpan` 2.0))

(event `self.ReceiveTick`
  (params (DeltaSeconds :type "Float (single-precision)"))
  (`self.K2_SetActorLocation` (+ (`self.K2_GetActorLocation`) (* (* (`KismetMathLibrary.Normal` (`self. Direction`)) (`self.Speed`)) DeltaSeconds))))

(fn `UserConstructionScript`)