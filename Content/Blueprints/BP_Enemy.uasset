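; BP_Enemy is an enemy actor that homes in on the player and destroys itself along with whatever it overlaps.
; BeginPlay finds the BP_Player actor and stores it as Target.
; Each Tick, FindDirection recomputes a normalized vector toward Target, replacing the initial downward direction, and the actor moves along it at Speed without sweeping.
; A begin overlap on the StaticMesh destroys both actors, with no filter on the other actor.
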(event `self.ReceiveBeginPlay`
  (bind _returnvalue (`GameplayStatics.GetActorOfClass` "/Game/Blueprints/BP_Player.BP_Player_C"))
  (set `self.Target` _returnvalue)
  (set `self.Direction` (`KismetMathLibrary.MakeVector` 0.0 0.0 -1.0)))

(event `self.ReceiveTick`
  (params (DeltaSeconds :type "Float (single-precision)"))
  (`self.FindDirection`)
  (`self.K2_SetActorLocation` (+ (`self.K2_GetActorLocation`) (* (* (`self.Direction`) (`self.Speed`)) DeltaSeconds))))

(event `self.StaticMesh.OnComponentBeginOverlap`
  (params (OverlappedComponent :type "PrimitiveComponent Object Reference") (OtherActor :type "Actor Object Reference") (OtherComp :type "PrimitiveComponent Object Reference") (OtherBodyIndex :type Integer) (bFromSweep :type Boolean) (SweepResult :type "HitResult Structure (by ref)"))
  ;[1 1 1] 충돌했을 때 너도 죽고 나도 죽고 싶다.
  (`self.K2_DestroyActor` OtherActor)
  (`self.K2_DestroyActor`))

(fn `FindDirection`
  (set `self.Direction` (`KismetMathLibrary.Normal` (- (`self.K2_GetActorLocation` (`self.Target`)) (`self.K2_GetActorLocation`)))))

(fn `UserConstructionScript`)